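; Pickup-style item actor that shows a Popup widget while the ThirdPersonCharacter overlaps it and destroys itself on that character's E press.
; Begin overlap caches the character, adds the widget to the viewport and sets Inrange; end overlap removes the widget and clears the flag.
; Tick polls the cached character's Epresses flag to trigger destruction, without checking Inrange.
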(event `self.ReceiveActorEndOverlap`
  (params (OtherActor :type "Actor Object Reference"))
  (`Widget.RemoveFromParent` (`self.NewVar_0`))
  (set `self.inrange` false))

(event `self.ReceiveActorBeginOverlap`
  (params (OtherActor :type "Actor Object Reference"))
  (bind _asthird_person_character (cast `/Game/ThirdPersonBP/Blueprints/ThirdPersonCharacter` OtherActor))
  (bind _returnvalue (`|CreateWidget` "/Game/UI/Popup.Popup_C"))
  (bind _output_get (set `self.NewVar_0` _returnvalue))
  (`UserWidget.AddToViewport` _output_get 0)
  (set `self.inrange` true))

(event `self.ReceiveTick`
  (params (DeltaSeconds :type "Float (single-precision)"))
  (if (`/Game/ThirdPersonBP/Blueprints/ThirdPersonCharacter.Epresses` (stale `self.ReceiveActorBeginOverlap` _asthird_person_character))
    (`self.K2_DestroyActor`)))

(fn `UserConstructionScript`)